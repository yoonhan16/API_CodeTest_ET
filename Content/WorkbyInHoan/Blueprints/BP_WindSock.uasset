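; BP_WindSock is a windsock actor whose wind direction and speed are set through an on-screen debug widget.
; BeginPlay creates the WindController widget hidden, and the F debug key toggles it along with the mouse cursor.
; Each Tick reads the rotation and speed sliders, yawing the Body to the direction and writing speed to the MPC_WeatherData parameter collection for materials to read.
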(event EventBeginPlay
  (bind _returnvalue (Game|GetPlayerController 0))
  ;[1 1 1] Show Widget in Viewport
  (Input|EnableInput _returnvalue)
  (bind _returnvalue_2 (UserInterface|CreateWidget "/Game/WorkbyInHoan/Widgets/WB_WindControllerWidget.WB_WindControllerWidget_C" _returnvalue))
  (Variables|Default|SetWindController _returnvalue_2)
  (UserInterface|Viewport|AddtoViewport (Variables|Default|GetWindController) 0)
  (Widget|SetVisibility (Variables|Default|GetWindController) "Hidden"))

(event EventTick
  (params (DeltaSeconds :type Float%20%28single-precision%29))
  (bind _windcontroller (Variables|Default|GetWindController))
  ;[1 1 1] Get Widget Data Value
  (CallFunction|RunWindSockbyWind (* (Class|Slider|GetValue (Variables|/Game/WorkbyInHoan/Widgets/WB_WindControllerWidget.WB_WindControllerWidget_C|GetRotationSlider _windcontroller)) 3.6e+02) (Class|Slider|GetValue (Variables|/Game/WorkbyInHoan/Widgets/WB_WindControllerWidget.WB_WindControllerWidget_C|GetSpeedSlider _windcontroller))))

(event Input|KeyboardEvents|DebugKeyF
  (params (Key :type Key%20Structure :default "None") (ActionValue :type Input%20Action%20Value%20Structure))
  (bind _returnvalue (Game|GetPlayerController 0))
  (bind _windcontroller (Variables|Default|GetWindController))
  (:Pressed
    ;[1 1 1] Press F, Widget On/Off
    (Utilities|FlowControl|FlipFlop
      (:A
        (Variables|/Script/Engine.PlayerController|SetbShowMouseCursor _returnvalue true)
        (Widget|SetVisibility _windcontroller "Visible"))
      (:B
        (Variables|/Script/Engine.PlayerController|SetbShowMouseCursor _returnvalue false)
        (Widget|SetVisibility _windcontroller "Hidden")))))

(fn ConstructionScript)

(fn RunWindSockbyWind
  (params (Wind%20Rotation :type Float%20%28single-precision%29) (WindSpeed :type Float%20%28single-precision%29))
  ;[1 1 1] Wind Direction
  (Transformation|SetRelativeRotation (Variables|Default|GetBody) (Math|Rotator|MakeRotator 0.0 0.0 Wind%20Rotation) false false)
  ;[1 1 1] Wind Speed
  (Rendering|Material|SetScalarParameterValue "/Game/MaterialParameterCollection/MPC_WeatherData.MPC_WeatherData" "Wind Speed" WindSpeed :!class /Script/Engine.KismetMaterialLibrary))