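; BP_WindSensor is a wind sensor prop with an arrow that points along a configured wind direction.
; The construction script calls RunFunctionByTheWind, which sets the Arrow component's relative yaw from WindDirectionZYaw.
; The arrow updates only at construction, as Tick is empty.
; Wing rotation logic, along with WindSpeed and TopBar yaw nodes, is left disconnected, so the wing does not spin.
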(event EventTick
  (params (DeltaSeconds :type Float%20%28single-precision%29)))

(fn ConstructionScript
  (CallFunction|RunFunctionbytheWind))

(fn RunFunctionbytheWind
  ;[1 1 1] Arrow Rotator by the Wind
  (Transformation|SetRelativeRotation (Variables|Default|GetArrow) (Math|Rotator|MakeRotator 0.0 0.0 (Math|Conversions|ToFloat(Integer) (Variables|Wind|GetWindDirection%20Z%28Yaw%29))) false false))